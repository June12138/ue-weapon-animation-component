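; BP_WeaponAnimComponent is an actor component that selects procedural weapon animation settings for its BP_FirstPersonCharacter owner.
; UpdateSettings applies named presets for sway, recoil, static and movement bob, and base pose, and adjusts bob and jump multipliers.
; Aiming or a playing ADS animation takes priority with ADS presets; otherwise the owner's stand, crouch or sprint stance picks the bob and base presets.
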(event `self.ReceiveBeginPlay`
  (bind _asbp_first_person_character (cast `/Game/FirstPerson/Blueprints/BP_FirstPersonCharacter` (`self.GetOwner`)))
  (set `self.Owner` _asbp_first_person_character))

(event `self.UpdateSettings`
  (if (or (`self.IsAiming`) (`self.PlayingADSAnimation`))
    (`self.SetSway` "ADSSway")
    (`self.SetRecoil` "ADSRecoil")
    (`self.SetStaticBob` "IdleBobADS")
    (`self.SetMovementBob` "WalkBobADS")
    (set `self.BobMultiplier` 0.1)
    (else
      (`self.SetRecoil` "DefaultRecoil")
      (`self.SetSway` "DefaultSway")
      (set `self.JumpMultiplier` 1.0)
      (switch `EStanceState` (`/Game/FirstPerson/Blueprints/BP_FirstPersonCharacter.CurrentStance` (`self.Owner`))
        (:`Stand`
          (`self.SetStaticBob` "IdleBob")
          (`self.SetMovementBob` "WalkBob")
          (`self.SetBase` "IdleBase")
          (set `self.BobMultiplier` 1.0))
        (:`Crouch`
          (`self.SetStaticBob` "IdleBob")
          (`self.SetMovementBob` "WalkBob")
          (`self.SetBase` "CrouchBase")
          (set `self.BobMultiplier` 0.7))
        (:`Sprint`
          (`self.SetMovementBob` "RunBob")
          (`self.SetBase` "SprintBase")
          (set `self.BobMultiplier` 1.0))))))

(fn `UpdateSettings_Old`)